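; BP_EnemySpawner is an actor that periodically spawns AI enemies at its own location.
; Tick accumulates time and, once SpawnTime elapses, resets it and passes a random Enemies entry to SpawnEnemy; the index range includes the array length, one past the last element.
; SpawnEnemy spawns the pawn and, if it is a BP_Enemy, calls MoveTo with the player character's location at that moment.
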(event `self.ReceiveBeginPlay`)

(event `self.ReceiveActorBeginOverlap`
  (params (OtherActor :type "Actor Object Reference")))

(event `self.ReceiveTick`
  (params (DeltaSeconds :type "Float (single-precision)"))
  (bind _enemies (`self.Enemies`))
  (bind _output_get (set `self.TimeSinceLastSpawn` (+ DeltaSeconds (`self.TimeSinceLastSpawn`))))
  (if (>= _output_get (`self.SpawnTime`))
    (set `self.TimeSinceLastSpawn` 0.0)
    (`self.SpawnEnemy` (`KismetArrayLibrary.Array_Get` _enemies (`KismetMathLibrary.RandomIntegerInRange` 0 (`KismetArrayLibrary.Array_Length` _enemies))))))

(fn `SpawnEnemy`
  (params (Enemy :type "/Game/Blueprints/BP_Enemy Class Reference"))
  (bind _returnvalue (`AIBlueprintHelperLibrary.SpawnAIFromClass` Enemy null (`self.K2_GetActorLocation`)))
  (bind _asbp_enemy (cast `/Game/Blueprints/BP_Enemy` _returnvalue))
  (`/Game/Blueprints/BP_Enemy.Move to` _asbp_enemy (`self.K2_GetActorLocation` (`GameplayStatics.GetPlayerCharacter` 0))))

(fn `UserConstructionScript`)