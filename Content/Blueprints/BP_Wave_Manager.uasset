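; BP_Wave_Manager is a timer-driven wave manager that starts a new wave at a fixed interval.
; Event Tick accumulates elapsed time, then resets it and calls SpawnWave once TimeBetweenWaves is reached.
; SpawnWave only increments CurrentWave and prints a debug message; no actors are spawned here.
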(event `self.ReceiveBeginPlay`)

(event `self.ReceiveActorBeginOverlap`
  (params (OtherActor :type "Actor Object Reference")))

(event `self.ReceiveTick`
  (params (DeltaSeconds :type "Float (single-precision)"))
  (bind _timesincelastwave (`self.TimeSinceLastWave`))
  (set `self.TimeSinceLastWave` (+ DeltaSeconds _timesincelastwave))
  (if (>= _timesincelastwave (`self.TimeBetweenWaves`))
    (set `self.TimeSinceLastWave` 0.0)
    (`self.SpawnWave`)))

(fn `SpawnWave`
  (set `self.CurrentWave` (+ (`self.CurrentWave`) 1))
  (`KismetSystemLibrary.PrintString` "Spawning wave"))

(fn `UserConstructionScript`)