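; Enemy actor that chases the player, shows its health in a widget and destroys itself at zero health.
; Each Tick records the player's location while within AggroRadius and always moves toward the last recorded location.
; Tick also pushes health values into the Enemy_Health widget, so the death check only runs if that cast succeeds.
; ApplyDamage subtracts from CurrentHealth, which starts at MaxHealth.
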(event `self.ReceiveBeginPlay`
  (set `self.CurrentHealth` (`self.MaxHealth`)))

(event `self.ReceiveTick`
  (params (DeltaSeconds :type "Float (single-precision)"))
  (bind _returnvalue (`GameplayStatics.GetPlayerCharacter` 0))
  (if (<= (`self.GetDistanceTo` _returnvalue) (`self.AggroRadius`))
    (set `self.LastPlayerLocation` (`self.K2_GetActorLocation` _returnvalue)))
  (`NavigationSystem.SimpleMoveToLocation` (`self.GetController`) (`self.LastPlayerLocation`))
  ;[1 1 1] Update UI health
  (bind _asenemy_health (cast `/Game/UMG/Enemy_Health` (`WidgetComponent.GetUserWidgetObject` (`self.Widget`))))
  (set `/Game/UMG/Enemy_Health.CurrentHealth` (`self.CurrentHealth`) _asenemy_health)
  (set `/Game/UMG/Enemy_Health.MaxHealth` (`self.MaxHealth`) _asenemy_health)
  (if (<= (`self.CurrentHealth`) 0.0)
    (`self.K2_DestroyActor`)))

(fn `Apply Damage`
  (params (DamageAmount :type "Float (double-precision)"))
  (set `self.CurrentHealth` (- (`self.CurrentHealth`) DamageAmount)))

(fn `UserConstructionScript`
  ;[1 1 1] Initialize
  (set `self.CurrentHealth` (`self.MaxHealth`)))