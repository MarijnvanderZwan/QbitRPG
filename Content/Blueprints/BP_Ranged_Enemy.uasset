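; Ranged enemy that chases the player within an aggro radius and fires skull fireballs when within shooting range.
; Tick-driven distance checks record the player's location and either move toward it, shoot, or turn to face the player during cooldown.
; ShootAt spawns BP_Skull_Fireball below the actor's origin aimed at the target; delays gate the next shot and follow-up move.
; An older cast-based attack chain remains in the graph, disconnected.
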(event `self.ReceiveTick`
  (params (DeltaSeconds :type "Float (single-precision)"))
  (bind _returnvalue (`GameplayStatics.GetPlayerCharacter` 0))
  (bind _lastplayerlocation (`self.LastPlayerLocation`))
  (bind _returnvalue_2 (`self.GetDistanceTo` _returnvalue))
  (if (<= _returnvalue_2 (`self.AggroRadius`))
    (set `self.LastPlayerLocation` (`self.K2_GetActorLocation` _returnvalue))
    (if (<= _returnvalue_2 (`self.ShootingRadius`))
      (if (`self.CanShoot`)
        (`self.ShootAt` _lastplayerlocation)
        (set `self.CanShoot` false)
        (`KismetSystemLibrary.Delay` 2.0)
        (set `self.CanShoot` true)
        (`KismetSystemLibrary.RetriggerableDelay` 0.6)
        (`|AIMoveTo` self (`self.LastPlayerLocation`) null (* (`self.ShootingRadius`) 0.75))
        (else
          (`self.SetActorRotation` (`KismetMathLibrary.FindLookAtRotation` (`self.K2_GetActorLocation`) (`self.K2_GetActorLocation` (`GameplayStatics.GetPlayerCharacter` 0))))))
      (else
        (`|AIMoveTo` self _lastplayerlocation null (* (`self.ShootingRadius`) 0.75))))))

(fn `ShootAt`
  (params (Target :type "Object.Vector Structure" :default (0.0 0.0 0.0)))
  (bind _returnvalue (`self.K2_GetActorLocation`))
  (`|SpawnActorFromClass` "/Game/Blueprints/BP_Skull_Fireball.BP_Skull_Fireball_C" (`KismetMathLibrary.MakeTransform` (- _returnvalue (0.0 0.0 100.0)) (`KismetMathLibrary.FindLookAtRotation` _returnvalue Target)) true))

(fn `UserConstructionScript`
  (`parent.UserConstructionScript`))