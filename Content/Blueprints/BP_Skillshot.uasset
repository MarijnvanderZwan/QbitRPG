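; BP_Skillshot is a skillshot indicator actor that shows an area of effect and damages enemies inside it when confirmed.
; The construction script applies the configured mesh, and LookAtPoint keeps it at the player's position at a set height, optionally yawing toward the mouse.
; ShotConfirmed uses the mesh itself as the hit shape, overlapping WorldDynamic objects and calling ApplyDamage on BP_Enemy hits.
; Its own ApplyDamage function is an empty stub.
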(fn `ApplyDamage`
  (params (Amount :type "Float (double-precision)")))

(fn `LookAtPoint`
  (params (`Player Location` :type "Object.Vector Structure") (`Mouse Location` :type "Object.Vector Structure"))
  (bind _returnvalue (`KismetMathLibrary.MakeVector` (.x `Player Location`) (.y `Player Location`) (`self.Height`)))
  ;[1 1 1] Turn indicator to point
  (`self.K2_SetActorRelativeLocation` _returnvalue)
  (if (`self.FollowsMouse`)
    (`self.SetActorRotation` (`KismetMathLibrary.MakeRot` 0.0 (.yaw (`KismetMathLibrary.FindLookAtRotation` _returnvalue `Mouse Location`))))))

(fn `ShotConfirmed`
  ;[1 1 1] Confirm skillshot
  (bind _outactors (`KismetSystemLibrary.ComponentOverlapActors_NEW` (`self.Mesh`) (`self.GetTransform`) (`|MakeArray` "ObjectTypeQuery2" :!type "EngineTypes.EObjectTypeQuery Enum")))
  (for _array_element _outactors
    (bind _asbp_enemy (cast `/Game/Blueprints/BP_Enemy` _array_element))
    (`/Game/Blueprints/BP_Enemy.Apply Damage` _asbp_enemy (`self.Damage`))))

(fn `UserConstructionScript`
  (`StaticMeshComponent.SetStaticMesh` (`self.Mesh`) (`self.SkillShotMesh`)))